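; BP_SafeZone is a zone actor that, despite its name, damages the first-person player standing inside it.
; Five seconds after BeginPlay it checks overlap once, and if the player is inside it spawns a Niagara effect and starts damage.
; The damage event re-arms its own looping timer, applying the full ZoneDPS value every 0.2 seconds.
; Leaving the collision clears that timer by function name, and re-entry does not restart it.
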(event `StartDamagingPlayer`
  (`KismetSystemLibrary.K2_SetTimerDelegate` (delegate `StartDamagingPlayer`) 0.2 true)
  (bind _asbp_first_person_character (cast `/Game/FirstPerson/Blueprints/BP_FirstPersonCharacter` (`GameplayStatics.GetPlayerPawn` 0)))
  (`GameplayStatics.ApplyDamage` _asbp_first_person_character (`KismetMathLibrary.Conv_IntToDouble` (`self.zoneDPS`)) null self))

(event `StopDamagingPlayer`
  (`KismetSystemLibrary.K2_ClearTimer` null "StartDamagingPlayer"))

(event `Play Niagara`
  (`NiagaraFunctionLibrary.SpawnSystemAtLocation` "/Game/Niagara/NS_SafeZone.NS_SafeZone" (`self.K2_GetActorLocation`)))

(event `self.ReceiveBeginPlay`
  (`KismetSystemLibrary.Delay` 5.0)
  (if (`PrimitiveComponent.IsOverlappingActor` (`self.ZoneCollision`) (`GameplayStatics.GetPlayerPawn` 0))
    (`self.Play Niagara`)
    (`self.StartDamagingPlayer`)))

(event `self.ZoneCollision.OnComponentEndOverlap`
  (params (OverlappedComponent :type "PrimitiveComponent Object Reference") (OtherActor :type "Actor Object Reference") (OtherComp :type "PrimitiveComponent Object Reference") (OtherBodyIndex :type Integer))
  (cast `/Game/FirstPerson/Blueprints/BP_FirstPersonCharacter` OtherActor)
  (`self.StopDamagingPlayer`))

(fn `UserConstructionScript`)
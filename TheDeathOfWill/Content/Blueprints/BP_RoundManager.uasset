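; Round manager that runs timed enemy waves, where surviving until the countdown expires counts as success.
; On BeginPlay it generates spawn points through BP_Spawner, creates the rounds HUD and starts the first round.
; Looping timers tick the countdown and spawn humanoid enemies at random points, with counts based on round number.
; Round end destroys enemies and broadcasts the result; success sets an intermission timer, failure opens DevTesting.
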(event `ShowUI`
  ; Create UI
  (bind _returnvalue (`|CreateWidget` "/Game/Blueprints/UI_RoundsHUD.UI_RoundsHUD_C"))
  (bind _output_get (set `self.HUDRef` _returnvalue))
  (`UserWidget.AddToViewport` _output_get 0))

(event `GenerateSapwns`
  ; Generate the SpawnPoints and get a reference to them
  (bind _outactors (`GameplayStatics.GetAllActorsOfClass` "/Game/Blueprints/BP_Spawner.BP_Spawner_C"))
  (bind _output (`|GetArrayItem` _outactors))
  (bind _output_get (set `/Game/Blueprints/BP_Spawner.SpawnPointsCount` (+ (`self.CurrentRound`) 2) _output))
  (`/Game/Blueprints/BP_Spawner.SpawnMultipleOfClass` _output "/Game/Blueprints/BP_SpawnPoint.BP_SpawnPoint_C" _output_get)
  (bind _outactors_2 (`GameplayStatics.GetAllActorsOfClass` "/Game/Blueprints/BP_SpawnPoint.BP_SpawnPoint_C"))
  (for _array_element _outactors_2
    (`KismetArrayLibrary.Array_AddUnique` (`self.SpawnPoints`) _array_element)))

(event `self.ReceiveBeginPlay`
  ; Start Round for the first tiem
  (`KismetSystemLibrary.Delay` 1.0)
  (`self.GenerateSapwns`)
  (`self.ShowUI`)
  (`self.StartRound`))

(event `StartRound`
  ; Round Start Logic
  (set `self.isRoundActive` true)
  (set `self.TimeRemaining` (`self.RoundDuration`))
  (bind _output_get (set `self.EnemiesToSpawn` (+ (+ (- (`self.CurrentRound`) 1) (`self.EnemiesPRoundIncrease`)) (`self.BaseEnemyCount`))))
  (set `self.SpawnsRemaining` _output_get)
  (set `self.EnemiesAlive` 0)
  (`self.StartEnemySpawn`)
  (bind _returnvalue (`KismetSystemLibrary.K2_SetTimer` null "RoundUpdate" 1.0 true))
  (set `self.RoundTimerHandle` _returnvalue)
  (`self.OnRoundStart`))

(event `RoundUpdate`
  ; Round Update Logic
  (bind _output_get (set `self.TimeRemaining` (- (`self.TimeRemaining`) 1.0)))
  (`self.OnRoundUpdate` _output_get)
  (if (<= (`self.TimeRemaining`) 0.0)
    (set `self.TimeRemaining` 0.0)
    (`self.EndRoundSuccess`)))

(event `EnemyDied`
  ; Logic for when an enemy is eliminated
  (set `self.EnemiesAlive` (- (`self.EnemiesAlive`) 1))
  (if (< (`self.EnemiesAlive`) 0)
    (set `self.EnemiesAlive` 0)))

(event `SpawnEnemy`
  ; Logic for the enemy spawns
  (if (> (`self.SpawnsRemaining`) 0)
    (`KismetSystemLibrary.Delay` 0.2)
    (`|SpawnActorFromClass` "/Game/Blueprints/BP_HumanoidEntity.BP_HumanoidEntity_C" (`self.GetTransform` (`|GetArrayItem` (`self.SpawnPoints`) (`KismetMathLibrary.RandomIntegerInRange` 0 (- (`KismetArrayLibrary.Array_Length` (`self.SpawnPoints`)) 1)))) "AdjustIfPossibleButAlwaysSpawn" "MultiplyWithRoot" null null)
    (set `self.SpawnsRemaining` (- (`self.SpawnsRemaining`) 1))
    (set `self.EnemiesAlive` (+ (`self.EnemiesAlive`) 1))
    (else
      (`KismetSystemLibrary.K2_ClearAndInvalidateTimerHandle` (`self.SpawnTimerHandle`)))))

(event `EndRoundSuccess`
  ; In case Rounded ended
  (set `self.isRoundActive` false)
  (`KismetSystemLibrary.K2_ClearAndInvalidateTimerHandle` (`self.RoundTimerHandle`))
  (`self.CleanUp Round`)
  (`self.OnRoundEnd` true (`self.CurrentRound`))
  (`KismetSystemLibrary.K2_SetTimerDelegate` (`|CreateDelegate` :!event `StartNextRound`) (`self.IntermissionDuration`)))

(event `EndRoundFail`
  ; In case Rounded ended
  (set `self.isRoundActive` false)
  (`KismetSystemLibrary.K2_ClearAndInvalidateTimerHandle` (`self.RoundTimerHandle`))
  (`self.CleanUp Round`)
  (`self.OnRoundEnd` false (`self.CurrentRound`))
  (`GameplayStatics.OpenLevel` "DevTesting"))

(event `CleanUp Round`
  ; Clean Up BPs elements before the new round starts
  (`KismetSystemLibrary.K2_ClearAndInvalidateTimerHandle` (`self.SpawnTimerHandle`))
  (bind _outactors (`GameplayStatics.GetAllActorsOfClass` "/Game/Blueprints/BP_HumanoidEntity.BP_HumanoidEntity_C"))
  (for _array_element _outactors
    (`self.K2_DestroyActor` _array_element)))

(event `StartNextRound`
  ; Logic for starting a new round
  (set `self.CurrentRound` (+ (`self.CurrentRound`) 1))
  (`self.StartRound`))

(fn `StartEnemySpawn`
  (bind _returnvalue (`KismetSystemLibrary.K2_SetTimer` null "SpawnEnemy" (`self.SpawnInterval`) true))
  (set `self.SpawnTimerHandle` _returnvalue))

(fn `UserConstructionScript`)
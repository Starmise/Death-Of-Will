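; BP_Spawner scatters WillItem pickups at random navigable points around its SpawnArea when play begins.
; A reusable function loops over a given class and count, querying the NavMesh within SpawnRadius for each instance.
; Actors spawn slightly above the found point, adjusting for collision but always spawning.
; Failed NavMesh queries are skipped without retry, so fewer items than requested may appear.
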(event `self.ReceiveBeginPlay`
  (`self.SpawnMultipleOfClass` "/Game/Blueprints/BP_WillItem.BP_WillItem_C" (`self.WillItemCount`)))

(fn `GetRandomPointInNavMesh`
  (returns (OutLocation :type "Vector Structure") (OutValue :type Boolean))
  ; Spawn Instances in random point of the NavMesh
  (bind (_randomlocation _returnvalue) (`NavigationSystemV1.K2_GetRandomLocationInNavigableRadius` (`SceneComponent.K2_GetComponentLocation` (`self.SpawnArea`)) (`self.SpawnRadius`) null null))
  (return _randomlocation _returnvalue))

(fn `SpawnMultipleOfClass`
  (params (ClassToSpawn :type "Actor Class Reference") (Count :type Integer))
  ; Spawning Multiple instances of a given BP
  (for _ (range Count)
    (bind (_outlocation _outvalue) (`self.GetRandomPointInNavMesh`))
    (if _outvalue
      (`|SpawnActorFromClass` ClassToSpawn (`KismetMathLibrary.MakeTransform` (`KismetMathLibrary.MakeVector` (.x _outlocation) (.y _outlocation) (+ (.z _outlocation) 10.0))) "AdjustIfPossibleButAlwaysSpawn" "MultiplyWithRoot" null null))))

(fn `UserConstructionScript`)